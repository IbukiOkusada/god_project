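; BP_GodCube is an actor that floats smoothly up and down in place.
; Each Tick adds the change in a sine of its lifetime over that frame, scaled to set the bob height, to its Z location.
; X and Y are left as they are, and the move neither sweeps nor teleports.
; A SetActorRotation node is present but never runs.
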(event `self.ReceiveTick`
  (params (DeltaSeconds :type "Float (single-precision)"))
  (bind _returnvalue (`self.GetGameTimeSinceCreation`))
  (set `self.Delta Seconds` DeltaSeconds)
  (`self.K2_SetActorLocation` (`KismetMathLibrary.MakeVector` (.x (`self.K2_GetActorLocation`)) (.y (`self.K2_GetActorLocation`)) (+ (.z (`self.K2_GetActorLocation`)) (* (- (`KismetMathLibrary.Sin` (+ _returnvalue (`self.Delta Seconds`))) (`KismetMathLibrary.Sin` _returnvalue)) 50.0)))))

(fn `UserConstructionScript`)